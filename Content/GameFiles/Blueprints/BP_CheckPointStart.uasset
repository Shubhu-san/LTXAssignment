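; BP_CheckPointStart is a checkpoint trigger that starts an on-screen timer when a VehicleAdvPawn enters its box.
; Each vehicle overlap creates and displays a new TimeUI widget; overlap by any other actor stops the timer.
; While running, Tick calls SetElapsedTime to accumulate delta seconds without resetting.
; A DoOnce reset after a Delay limits whole-second text updates to about once per second.
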(event `self.ReceiveBeginPlay`)

(event `self.ReceiveTick`
  (params (DeltaSeconds :type "Float (single-precision)"))
  (`self.SetElapsedTime`))

(event `self.Box.OnComponentBeginOverlap`
  (params (OverlappedComponent :type "PrimitiveComponent Object Reference") (OtherActor :type "Actor Object Reference") (OtherComp :type "PrimitiveComponent Object Reference") (OtherBodyIndex :type Integer) (bFromSweep :type Boolean) (SweepResult :type "HitResult Structure (by ref)"))
  (cast `/Game/GameFiles/Blueprints/VehicleAdvPawn` OtherActor
    (:`then`
      (bind _returnvalue (`|CreateWidget` "/Game/GameFiles/Blueprints/TimeUI.TimeUI_C" (`GameplayStatics.GetPlayerController` 0)))
      (bind _output_get (set `self.UI` _returnvalue))
      (`UserWidget.AddToViewport` _output_get 0)
      (set `self.StartTimer` true))
    (:`CastFailed`
      (set `self.StartTimer` false))))

(fn `UserConstructionScript`)